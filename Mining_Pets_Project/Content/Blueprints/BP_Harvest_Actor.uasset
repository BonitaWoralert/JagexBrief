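; Harvestable ore actor that the player or pet AI mines for resources.
; Clicking nearby starts player mining; hovered right-click opens a Tick gate that sends the pet over to mine.
; Looping timers count random waits, cancel on movement, roll for resources and deplete ore health until a destructible replacement crumbles.
; Player harvests build pet charge; clicking at full charge triggers an ice blast that destroys the ore for bonus resources.
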(event OnClicked(StaticMesh)
  (params (TouchedComponent :type Primitive%20Component%20Object%20Reference) (ButtonPressed :type Key%20Structure :default "None"))
  ;[1 1 1] Check whether the player is close enough to the ORE, then play the mining animation and begin harvesting.
  (if (>= (Variables|/Game/TopDownBP/Blueprints/TopDownCharacter.TopDownCharacter_C|GetPetAbilityCharge (Variables|Default|GetCharacterReference)) 1.0)
    (|SpecialAttack)
    (elif (< (Transformation|GetDistanceTo (Game|GetPlayerCharacter 0)) 4e+02)
      (CallFunction|RotatePlayertoHarvest)
      (Development|PrintString "Harvest Started!")
      (Components|Animation|PlayAnimation (Variables|/Script/Engine.Character|GetMesh (Variables|Default|GetCharacterReference)) "/Game/Animations/StandingMeleeAttackDownward_3_4UE4.StandingMeleeAttackDownward_3_4UE4" true)
      (CallFunction|DetermineWaitTime)
      (bind _returnvalue (Utilities|Time|SetTimerbyFunctionName 0 "Harvest" (Utilities|Time|GetWorldDeltaSeconds) true))
      (Variables|Default|SetharvestTimerHandle _returnvalue))))

(event OnBeginCursorOver(StaticMesh)
  (params (TouchedComponent :type Primitive%20Component%20Object%20Reference))
  (Variables|Default|SetHoveringOnOre? true))

(event OnEndCursorOver(StaticMesh)
  (params (TouchedComponent :type Primitive%20Component%20Object%20Reference))
  (Variables|Default|SetHoveringOnOre? false))

(event EventBeginPlay
  (bind _returnvalue (Actor|GetActorOfClass "/Game/Blueprints/AI/Pet_AI.Pet_AI_C"))
  (bind _aspet_ai (Utilities|Casting|CastToPet_AI _returnvalue))
  (Variables|Default|SetPet_AI_Ref _aspet_ai))

(event EventTick
  (params (DeltaSeconds :type Float%20%28single-precision%29))
  (bind _pet_ai_ref (Variables|Default|GetPet_AI_Ref))
  (Default|FollowPlayer (Variables|Default|GetPet_AI_Ref))
  (Utilities|FlowControl|Sequence
    (:then_0
      (Utilities|FlowControl|Gate true :!label _label
        (:Exit
          (Variables|/Game/Blueprints/AI/Pet_AI.Pet_AI_C|SetFollowPlayer _pet_ai_ref false)
          (if (< (Transformation|GetDistanceTo _pet_ai_ref) 2e+02)
            (while (Variables|Default|GetKeepHarvesting?)
              (Variables|Default|SetKeepHarvesting? false)
              (CallFunction|RotateAItoHarvest)
              (Development|PrintString "AI Harvest Started!" true true "(R=0.000000,G=0.660000,B=1.000000,A=1.000000)" 0.0)
              (Components|Animation|PlayAnimation (Variables|/Script/Engine.Character|GetMesh (Variables|Default|GetPet_AI_Ref)) "/Game/Animations/StandingMeleeAttackDownward_3_4UE4.StandingMeleeAttackDownward_3_4UE4" true)
              (CallFunction|DetermineWaitTimeAI)
              (bind _returnvalue (Utilities|Time|SetTimerbyFunctionName 0 "AI_Harvest" (Utilities|Time|GetWorldDeltaSeconds) true))
              (Variables|Default|SetAI_harvestTimerHandle _returnvalue)
              (Utilities|FlowControl|Delay (Variables|Default|GetAI_waitTime))
              (Variables|Default|SetKeepHarvesting? true))
            (else
              (AI|AIMoveTo (Variables|Default|GetPet_AI_Ref) "0, 0, 0" self 5.0 false))))))
    (:then_1
      (|CharacterRef)
      (if (Variables|Default|GetHoveringOnOre?)
        (if (Variables|/Game/TopDownBP/Blueprints/TopDownCharacter.TopDownCharacter_C|GetRightMouseButtonClicked? (Variables|Default|GetCharacterReference))
          (Variables|Default|SetShouldGATECONTINUE? true)
          (goto _label Open))))
    (:then_2
      (if (not (Variables|Default|GetShouldGATECONTINUE?))
        (goto _label Close)))))

(fn ConstructionScript)

(fn DetermineWaitTime
  (bind _harvestwaitrange (Variables|Default|GetharvestWaitRange))
  ;[1 1 1] Set the harvest time as a random time within the harvest wait range.
  (Variables|Default|SetwaitTime (Math|Random|RandomFloatinRange (Utilities|Array|Get(acopy) _harvestwaitrange) (Utilities|Array|Get(acopy) _harvestwaitrange 1))))

(fn Harvest
  (bind _characterreference (Variables|Default|GetCharacterReference))
  (bind _characterreference_2 (Variables|Default|GetCharacterReference))
  (bind _characterreference_3 (Variables|Default|GetCharacterReference))
  (bind _petabilitychargechance (Variables|Default|GetPetAbilityChargeChance))
  (bind _resourcechance (Variables|Default|GetresourceChance))
  (bind _mesh (Variables|/Script/Engine.Character|GetMesh _characterreference_2))
  (bind _mesh_2 (Variables|/Script/Engine.Character|GetMesh _characterreference_3))
  ;[1 1 1] Check whether the harvest time is over
  (if (> (Variables|Default|GetcurrentTime) (Variables|Default|GetwaitTime))
    ;[1 1 1] Stop the pickaxe animation when the harvest is complete, if the player has gained a resource plus 1 to resources, if not print NO RESOURCES GAINED.
    (Development|PrintString "Harvest Complete")
    (Math|Integer|DecrementInt (Variables|Default|GetOreHealth)
      (:%20%20
        (Audio|Components|Audio|Stop _mesh)
        (Components|Animation|SetAnimationMode _mesh "AnimationBlueprint")
        (Variables|/Game/TopDownBP/Blueprints/TopDownCharacter.TopDownCharacter_C|SetPetAbilityCharge _characterreference (+ (Variables|/Game/TopDownBP/Blueprints/TopDownCharacter.TopDownCharacter_C|GetPetAbilityCharge _characterreference) (Math|Random|RandomFloatinRange (Utilities|Array|Get(acopy) _petabilitychargechance) (Utilities|Array|Get(acopy) _petabilitychargechance 1))))
        (if (== (Variables|Default|GetOreHealth) 0)
          (CallFunction|Destroy&Crumble)
          (Variables|Default|SetOreHealth (Variables|Default|GetDefaultOreHealth)))
        (if (>= (Math|Random|RandomIntegerinRange (Utilities|Array|Get(acopy) _resourcechance) (Utilities|Array|Get(acopy) _resourcechance 1)) (Utilities|Array|Get(acopy) _resourcechance 2))
          (bind _astop_down_character (Utilities|Casting|CastToTopDownCharacter (Game|GetPlayerCharacter 0)))
          (Math|Integer|IncrementInt (Variables|/Game/TopDownBP/Blueprints/TopDownCharacter.TopDownCharacter_C|GetResources _astop_down_character)
            (:%20%20
              _))
          (else
            (Development|PrintString "NO RESOURCES GAINED")))
        ;[1 1 1] Reset the timer.
        (Variables|Default|SetcurrentTime 0.0 :!label _label)
        (Utilities|Time|ClearandInvalidateTimerbyHandle (Variables|Default|GetharvestTimerHandle))))
    (else
      ;[1 1 1] Check whether the player is moving and if they are, cancel the harvest and stop animations.
      (if (Math|Vector|NotEqual(Vector) (Variables|/Script/Engine.MovementComponent|GetVelocity (Pawn|GetMovementComponent (Game|GetPlayerCharacter 0))) "0, 0, 0" 0.0001)
        (Development|PrintString "Harvest Cancelled")
        (Audio|Components|Audio|Stop _mesh_2)
        (Components|Animation|SetAnimationMode _mesh_2 "AnimationBlueprint")
        (goto _label)
        (else
          ;;[1 1 1] Set the current time to real world seconds, NOT IN GAME TICKS.
          (Variables|Default|SetcurrentTime (+ (Variables|Default|GetcurrentTime) (Utilities|Time|GetWorldDeltaSeconds))))))))

(fn RotatePlayertoHarvest
  (bind _characterreference (Variables|Default|GetCharacterReference))
  (bind _capsulecomponent (Variables|/Script/Engine.Character|GetCapsuleComponent _characterreference))
  ;[1 1 1] See where the player is rotated, and then rotate them towards the ORE.
  (Transformation|SetWorldRotation _capsulecomponent (Math|Rotator|MakeRotator 0.0 0.0 (.yaw (Math|Rotator|FindLookatRotation (Transformation|GetWorldLocation _capsulecomponent) (Transformation|GetWorldLocation (Variables|Default|GetStaticMesh))))) false false))

(fn Destroy&Crumble
  (|Destroy&Crumble_2))

(fn RotateAItoHarvest
  (bind _pet_ai_ref (Variables|Default|GetPet_AI_Ref))
  (bind _capsulecomponent (Variables|/Script/Engine.Character|GetCapsuleComponent _pet_ai_ref))
  ;[1 1 1] See where the player is rotated, and then rotate them towards the ORE.
  (Transformation|SetWorldRotation _capsulecomponent (Math|Rotator|MakeRotator 0.0 0.0 (.yaw (Math|Rotator|FindLookatRotation (Transformation|GetWorldLocation _capsulecomponent) (Transformation|GetWorldLocation (Variables|Default|GetStaticMesh))))) false false))

(fn DetermineWaitTimeAI
  (bind _ai_harvestwaitrange (Variables|Default|GetAI_harvestWaitRange))
  ;[1 1 1] Set the harvest time as a random time within the harvest wait range.
  (Variables|Default|SetAI_waitTime (Math|Random|RandomFloatinRange (Utilities|Array|Get(acopy) _ai_harvestwaitrange) (Utilities|Array|Get(acopy) _ai_harvestwaitrange 1))))

(fn AIHarvest
  (bind _pet_ai_ref (Variables|Default|GetPet_AI_Ref))
  (bind _pet_ai_ref_2 (Variables|Default|GetPet_AI_Ref))
  (bind _pet_ai_ref_3 (Variables|Default|GetPet_AI_Ref))
  (bind _resourcechance (Variables|Default|GetresourceChance))
  (bind _mesh (Variables|/Script/Engine.Character|GetMesh _pet_ai_ref))
  (bind _mesh_2 (Variables|/Script/Engine.Character|GetMesh _pet_ai_ref_2))
  ;[1 1 1] Check whether the harvest time is over
  (if (> (Variables|Default|GetAI_currentTime) (Variables|Default|GetAI_waitTime))
    ;[1 1 1] Stop the pickaxe animation when the harvest is complete, if the player has gained a resource plus 1 to resources, if not print NO RESOURCES GAINED.
    (Development|PrintString "Harvest Complete")
    (Math|Integer|DecrementInt (Variables|Default|GetOreHealth)
      (:%20%20
        (Audio|Components|Audio|Stop _mesh_2)
        (Components|Animation|SetAnimationMode _mesh_2 "AnimationBlueprint")
        (if (== (Variables|Default|GetOreHealth) 0)
          (CallFunction|Destroy&Crumble)
          (Variables|Default|SetShouldGATECONTINUE? false)
          (Variables|/Game/Blueprints/AI/Pet_AI.Pet_AI_C|SetFollowPlayer _pet_ai_ref_3 true)
          (Default|FollowPlayer _pet_ai_ref_3)
          (Variables|Default|SetOreHealth (Variables|Default|GetDefaultOreHealth)))
        (if (>= (Math|Random|RandomIntegerinRange (Utilities|Array|Get(acopy) _resourcechance) (Utilities|Array|Get(acopy) _resourcechance 1)) (Utilities|Array|Get(acopy) _resourcechance 2))
          (bind _astop_down_character (Utilities|Casting|CastToTopDownCharacter (Game|GetPlayerCharacter 0)))
          (Math|Integer|IncrementInt (Variables|/Game/TopDownBP/Blueprints/TopDownCharacter.TopDownCharacter_C|GetResources _astop_down_character)
            (:%20%20
              _))
          (else
            (Development|PrintString "NO RESOURCES GAINED")))
        ;[1 1 1] Reset the timer.
        (Variables|Default|SetAI_currentTime 0.0 :!label _label)
        (Utilities|Time|ClearandInvalidateTimerbyHandle (Variables|Default|GetAI_harvestTimerHandle))))
    (else
      ;[1 1 1] Check whether the player is moving and if they are, cancel the harvest and stop animations.
      (if (Math|Vector|NotEqual(Vector) (Variables|/Script/Engine.MovementComponent|GetVelocity (Pawn|GetMovementComponent (Variables|Default|GetPet_AI_Ref))) "0, 0, 0" 0.0001)
        (Audio|Components|Audio|Stop _mesh)
        (Components|Animation|SetAnimationMode _mesh "AnimationBlueprint")
        (Variables|Default|SetShouldGATECONTINUE? false)
        (goto _label)
        (else
          ;;[1 1 1] Set the current time to real world seconds, NOT IN GAME TICKS.
          (Variables|Default|SetAI_currentTime (+ (Variables|Default|GetAI_currentTime) (Utilities|Time|GetWorldDeltaSeconds))))))))