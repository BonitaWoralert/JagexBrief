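; Pet AI that follows the player's TopDownCharacter, cached on BeginPlay.
; A self-calling FollowPlayer event re-checks distance every 0.2 seconds, moving toward the player when far and targeting itself when close to hold position.
; The loop runs only while the FollowPlayer flag is true and has no restart once it stops.
; An unconnected node would attach PickFBX to the mesh's right-hand socket.
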(event Custom|Follow%20Player
  (if (Variables|Default|GetFollowPlayer)
    (if (>= (Transformation|GetDistanceTo (Variables|Default|GetCharacterReference)) 3e+02)
      (AI|AIMoveTo self "0, 0, 0" (Variables|Default|GetCharacterReference) 5.0 false
        (:then
          _))
      (else
        (AI|AIMoveTo self "0, 0, 0" self 5.0 false
          (:then
            _))))
    (Utilities|FlowControl|Delay 0.2)
    (CallFunction|FollowPlayer)))

(event EventBeginPlay
  (bind _astop_down_character (Utilities|Casting|CastToTopDownCharacter (Game|GetPlayerCharacter 0)))
  (Variables|Default|SetCharacterReference _astop_down_character)
  (CallFunction|FollowPlayer))

(fn ConstructionScript)